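; BP_Puerta is an interactive door that the player swings open by pressing Q while standing near it.
; Overlap of its Box by Character_BP enables input and shows an Interact widget; leaving disables input and removes it.
; Q runs a FlipFlop into the AnimPuerta timeline, which lerps the Arrow's yaw from PuertaCerrada to PuertaAbierta.
; Only the FlipFlop's A output is wired, so no closing path exists.
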(event `Key|Q`
  (params (Key :type "Key Structure"))
  (:`Pressed`
    (`/Engine/EditorBlueprintResources/StandardMacros.FlipFlop`
      (:`A`
        (bind (_direction _animacionpuerta) (`Timeline|anim puerta`)
          (:`Update`
            (`SceneComponent.K2_SetRelativeRotation` (`self.Arrow`) (`KismetMathLibrary.MakeRotator` 0.0 0.0 (`KismetMathLibrary.Lerp` (`self.Puerta cerrada`) (`self.Puerta abierta`) _animacionpuerta)) false false)))))))

(event `self.Box.OnComponentBeginOverlap`
  (params (OverlappedComponent :type "PrimitiveComponent Object Reference") (OtherActor :type "Actor Object Reference") (OtherComp :type "PrimitiveComponent Object Reference") (OtherBodyIndex :type Integer) (bFromSweep :type Boolean) (SweepResult :type "HitResult Structure (by ref)"))
  ;[1 1 1] mensaje interfaz
  (cast `/Game/BluePrints/Character_BP` OtherActor)
  (`self.EnableInput` (`GameplayStatics.GetPlayerController` 0))
  (bind _returnvalue (`|CreateWidget` "/Game/Added/CosasSalas/Interact.Interact_C"))
  (`UserWidget.AddToViewport` _returnvalue 0))

(event `self.Box.OnComponentEndOverlap`
  (params (OverlappedComponent :type "PrimitiveComponent Object Reference") (OtherActor :type "Actor Object Reference") (OtherComp :type "PrimitiveComponent Object Reference") (OtherBodyIndex :type Integer))
  ;[1 1 1] mensaje interfaz
  (cast `/Game/BluePrints/Character_BP` OtherActor)
  (`self.DisableInput` (`GameplayStatics.GetPlayerController` 0))
  (`Widget.RemoveFromParent` (stale `self.Box.OnComponentBeginOverlap` _returnvalue)))

(fn `UserConstructionScript`)