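; Test actor for a pushable box that flags player characters as pushing while they stand in its side triggers.
; Separate X-axis and Y-axis overlap volumes handle Character_BP identically, setting its Pushing flag on begin overlap and clearing it on end.
; Every overlap event also enables physics simulation on the box body, and nothing turns it back off or constrains movement per axis in this graph.
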(event `self.BoxYaxis.OnComponentBeginOverlap`
  (params (OverlappedComponent :type "PrimitiveComponent Object Reference") (OtherActor :type "Actor Object Reference") (OtherComp :type "PrimitiveComponent Object Reference") (OtherBodyIndex :type Integer) (bFromSweep :type Boolean) (SweepResult :type "HitResult Structure (by ref)"))
  ;[1 1 1] Y axis
  (bind _ascharacter_bp (cast `/Game/PiRats/BluePrints/Character_BP` OtherActor))
  (`PrimitiveComponent.SetSimulatePhysics` (`self.BoxBody`) true)
  (set `/Game/PiRats/BluePrints/Character_BP.Pushing` true _ascharacter_bp))

(event `self.BoxYaxis.OnComponentEndOverlap`
  (params (OverlappedComponent :type "PrimitiveComponent Object Reference") (OtherActor :type "Actor Object Reference") (OtherComp :type "PrimitiveComponent Object Reference") (OtherBodyIndex :type Integer))
  ;[1 1 1] Y axis
  (bind _ascharacter_bp (cast `/Game/PiRats/BluePrints/Character_BP` OtherActor))
  (`PrimitiveComponent.SetSimulatePhysics` (`self.BoxBody`) true)
  (set `/Game/PiRats/BluePrints/Character_BP.Pushing` false _ascharacter_bp))

(event `self.BoxXaxis.OnComponentBeginOverlap`
  (params (OverlappedComponent :type "PrimitiveComponent Object Reference") (OtherActor :type "Actor Object Reference") (OtherComp :type "PrimitiveComponent Object Reference") (OtherBodyIndex :type Integer) (bFromSweep :type Boolean) (SweepResult :type "HitResult Structure (by ref)"))
  (bind _ascharacter_bp (cast `/Game/PiRats/BluePrints/Character_BP` OtherActor))
  (`PrimitiveComponent.SetSimulatePhysics` (`self.BoxBody`) true)
  (set `/Game/PiRats/BluePrints/Character_BP.Pushing` true _ascharacter_bp))

(event `self.BoxXaxis.OnComponentEndOverlap`
  (params (OverlappedComponent :type "PrimitiveComponent Object Reference") (OtherActor :type "Actor Object Reference") (OtherComp :type "PrimitiveComponent Object Reference") (OtherBodyIndex :type Integer))
  (bind _ascharacter_bp (cast `/Game/PiRats/BluePrints/Character_BP` OtherActor))
  (`PrimitiveComponent.SetSimulatePhysics` (`self.BoxBody`) true)
  (set `/Game/PiRats/BluePrints/Character_BP.Pushing` false _ascharacter_bp))

(fn `UserConstructionScript`)